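; Left-hand door item that toggles open and closed when interacted with.
; The construction script stores the root's world rotation as the closed baseline.
; OnInteract flips DoorIsOpen and plays or reverses the Door_Open timeline, whose Door track drives a negative yaw offset from that baseline, applied as the actor's relative rotation.
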(event EventOnInteract
  (bind _rot (Variables|Default|GetRot))
  (bind (_roll _pitch _yaw) (Math|Rotator|BreakRotator _rot))
  ;[1 1 1] Door Open
  (if (Variables|Default|GetDoorIsOpen)
    (Variables|Default|SetDoorIsOpen false)
    (bind _door (Timeline|Door_Open Reverse)
      (:Update
        (Transformation|SetActorRelativeRotation (Math|Rotator|MakeRotator _roll _pitch (+ (* (/ _door 1e+01) -9e+01) _yaw)))))
    (else
      (Variables|Default|SetDoorIsOpen true)
      (Timeline|Door_Open Play))))

(fn ConstructionScript
  (Variables|Default|SetRot (Transformation|GetWorldRotation (Variables|Default|GetDefaultSceneRoot))))