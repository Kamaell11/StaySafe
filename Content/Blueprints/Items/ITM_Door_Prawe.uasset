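; Interactive door item that the player opens and closes with the Action input while inside its trigger.
; Trigger overlap enables and disables input for player controller 0, and each press flips DoorIsOpen to play or reverse the Door_Open timeline.
; The timeline's Door track sets the whole actor's yaw as an absolute rotation and prints that rotation as debug output.
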(event OnComponentBeginOverlap(Trigger)
  (params (OverlappedComponent :type Primitive%20Component%20Object%20Reference) (OtherActor :type Actor%20Object%20Reference) (OtherComp :type Primitive%20Component%20Object%20Reference) (OtherBodyIndex :type Integer) (bFromSweep :type Boolean) (SweepResult :type Hit%20Result%20Structure%20%28by%20ref%29))
  ;[1 1 1] Door Open
  (Input|EnableInput (Game|GetPlayerController 0)))

(event OnComponentEndOverlap(Trigger)
  (params (OverlappedComponent :type Primitive%20Component%20Object%20Reference) (OtherActor :type Actor%20Object%20Reference) (OtherComp :type Primitive%20Component%20Object%20Reference) (OtherBodyIndex :type Integer))
  ;[1 1 1] Door Open
  (Input|DisableInput (Game|GetPlayerController 0)))

(event Input|ActionEvents|InputActionAction
  (params (Key :type Key%20Structure :default "AnyKey"))
  ;[1 1 1] Door Open
  (:Pressed
    (if (Variables|Default|GetDoorIsOpen)
      (Variables|Default|SetDoorIsOpen false)
      (bind _door (Timeline|Door_Open Reverse)
        (:Update
          (Development|PrintString (Utilities|String|ToString(Rotator) (Math|Rotator|MakeRotator 0.0 0.0 _door)))
          (Transformation|SetActorRotation (Math|Rotator|MakeRotator 0.0 0.0 _door))))
      (else
        (Variables|Default|SetDoorIsOpen true)
        (Timeline|Door_Open Play)))))

(fn ConstructionScript)