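; TV item that plays the video and audio of a default VHS tape when play begins.
; On BeginPlay it takes the screen material, media sound cue, media player and source from DefaultVHS, applies them to the Screen and SoundCue, and opens the source.
; The construction script gives the Screen a plane material until play starts.
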(event EventBeginPlay
  (bind _default_vhs (Variables|Default|GetDefault%20VHS))
  (Rendering|Material|SetMaterial (Variables|Default|GetScreen) 0 (Variables|/Game/Blueprints/Items/ITM_VHS_Parent.ITM_VHS_Parent_C|GetScreen%20Material _default_vhs))
  (Audio|Components|Audio|SetSound (Variables|Default|GetSound_Cue) (Variables|/Game/Blueprints/Items/ITM_VHS_Parent.ITM_VHS_Parent_C|GetMedia%20Sound%20Cue _default_vhs))
  (Media|MediaPlayer|OpenSource (Variables|/Game/Blueprints/Items/ITM_VHS_Parent.ITM_VHS_Parent_C|GetMedia%20Player _default_vhs) (Variables|/Game/Blueprints/Items/ITM_VHS_Parent.ITM_VHS_Parent_C|GetMedia%20Source _default_vhs)))

(fn ConstructionScript
  (Rendering|Material|SetMaterial (Variables|Default|GetScreen) 0 "/Game/Textures/Items/TV/Material_Plane.Material_Plane"))