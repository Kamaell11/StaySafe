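; ITM_Door_lewe2 is an interactive door that the player swings open and closed with the Action input.
; A trigger component enables input for the first player controller on begin overlap and disables it on end overlap.
; Each press toggles DoorIsOpen and plays or reverses the Door_Open timeline, whose track is scaled into a yaw offset.
; That offset is added to the root's world rotation, cached in the construction script, and applied as the actor's relative rotation.
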(event OnComponentBeginOverlap(Trigger)
  (params (OverlappedComponent :type Primitive%20Component%20Object%20Reference) (OtherActor :type Actor%20Object%20Reference) (OtherComp :type Primitive%20Component%20Object%20Reference) (OtherBodyIndex :type Integer) (bFromSweep :type Boolean) (SweepResult :type Hit%20Result%20Structure%20%28by%20ref%29))
  ;[1 1 1] Door Open
  (Input|EnableInput (Game|GetPlayerController 0)))

(event OnComponentEndOverlap(Trigger)
  (params (OverlappedComponent :type Primitive%20Component%20Object%20Reference) (OtherActor :type Actor%20Object%20Reference) (OtherComp :type Primitive%20Component%20Object%20Reference) (OtherBodyIndex :type Integer))
  ;[1 1 1] Door Open
  (Input|DisableInput (Game|GetPlayerController 0)))

(event Input|ActionEvents|InputActionAction
  (params (Key :type Key%20Structure :default "AnyKey"))
  (bind _rot (Variables|Default|GetRot))
  (bind (_roll _pitch _yaw) (Math|Rotator|BreakRotator _rot))
  ;[1 1 1] Door Open
  (:Pressed
    (if (Variables|Default|GetDoorIsOpen)
      (Variables|Default|SetDoorIsOpen false)
      (bind _door (Timeline|Door_Open Reverse)
        (:Update
          (Transformation|SetActorRelativeRotation (Math|Rotator|MakeRotator _roll _pitch (+ (* (/ _door 1e+01) 9e+01) _yaw)))))
      (else
        (Variables|Default|SetDoorIsOpen true)
        (Timeline|Door_Open Play)))))

(fn ConstructionScript
  (Variables|Default|SetRot (Transformation|GetWorldRotation (Variables|Default|GetDefaultSceneRoot))))